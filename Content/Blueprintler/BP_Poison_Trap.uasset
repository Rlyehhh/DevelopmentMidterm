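; BP_Poison_Trap is a gas trap that repeatedly damages the first-person character while it overlaps the trap.
; Overlap begin starts a looping timer that applies PoisonDamage through DamageFunction, and any overlap end clears it by function name.
; It destroys itself when the level's Gas_Trap_Disabler fires TrapsDisabled.
; The construction script sizes its cube and box from the parent BP_Platfrom_Cell's grid size and wall height.
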(event `self.ReceiveBeginPlay`
  (bind _returnvalue (`GameplayStatics.GetActorOfClass` "/Game/Blueprintler/Gas_Trap_Disabler.Gas_Trap_Disabler_C"))
  (add `/Game/Blueprintler/Gas_Trap_Disabler.Traps_Disabled` _returnvalue (delegate `Disabled`)))

(event `Disabled`
  (`self.K2_DestroyActor`))

(event `self.ReceiveActorEndOverlap`
  (params (OtherActor :type "Actor Object Reference"))
  (`KismetSystemLibrary.K2_ClearTimer` null "Poison_Tick"))

(event `self.ReceiveActorBeginOverlap`
  (params (OtherActor :type "Actor Object Reference"))
  (bind _asbp_first_person_character (cast `/Game/FirstPerson/Blueprints/BP_FirstPersonCharacter` OtherActor))
  (set `self.As BP First Person Character` _asbp_first_person_character)
  (`KismetSystemLibrary.K2_SetTimerDelegate` (delegate `Poison_Tick`) 0.1 true))

(event `Poison_Tick`
  (`/Game/FirstPerson/Blueprints/BP_FirstPersonCharacter.Damage_Function` (`self.As BP First Person Character`) (`self.Poison_Damage`)))

(fn `UserConstructionScript`
  (bind _box (`self.Box`))
  (bind _asbp_platfrom_cell (cast `/Game/Blueprintler/BP_Platfrom_Cell` (`self.GetParentActor`)))
  (bind _returnvalue (* (`/Game/Blueprintler/BP_Platfrom_Cell.GridSize` _asbp_platfrom_cell) 1.0))
  (`SceneComponent.SetRelativeScale3D` (`self.Cube`) (`KismetMathLibrary.MakeVector` _returnvalue _returnvalue 0.1))
  (bind _wall_height (`/Game/Blueprintler/BP_Platfrom_Cell.wall_height` _asbp_platfrom_cell))
  (`SceneComponent.SetRelativeScale3D` _box (`KismetMathLibrary.MakeVector` _returnvalue _returnvalue _wall_height))
  (`SceneComponent.K2_SetRelativeLocation` _box (`KismetMathLibrary.MakeVector` 0.0 0.0 (* _wall_height 50.0)) false false))