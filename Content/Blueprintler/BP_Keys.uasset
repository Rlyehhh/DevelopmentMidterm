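; BP_Keys is a color-coded key pickup that bobs and spins through a looping timeline.
; The construction script sets the key's material and name from its Color (red, green or blue).
; Interact adds that name to the BP_FirstPersonCharacter's Keys, prints an acquisition message and destroys the actor.
; GetInteractState always returns false.
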(event `self.ReceiveBeginPlay`
  (bind _key (`self.key`))
  (bind (_relativelocation_x _relativelocation_y _relativelocation_z) (`KismetMathLibrary.BreakVector` (`SceneComponent.RelativeLocation` _key)))
  (bind _returnvalue (`GameplayStatics.GetActorOfClass` "/Game/FirstPerson/Blueprints/BP_FirstPersonCharacter.BP_FirstPersonCharacter_C"))
  (set `self.PlayerRef` _returnvalue)
  (bind (_direction _up_down _rotate) (`Timeline|Animation` :!label _label)
    (:`Update`
      (`SceneComponent.K2_SetRelativeLocation` _key (`KismetMathLibrary.MakeVector` _relativelocation_x _relativelocation_y (- _relativelocation_z _up_down)) false false)
      (bind _returnvalue_2 (* _rotate 90.0))
      (`SceneComponent.K2_SetRelativeRotation` _key (`KismetMathLibrary.MakeRotator` 0.0 _returnvalue_2 _returnvalue_2) false false))
    (:`Finished`
      (goto _label :!via `PlayFromStart`))))

(event `/Game/FirstPerson/Blueprints/Interface_Test.Interact`
  (bind _keycolorname (`self.KeyColorName`))
  (`KismetArrayLibrary.Array_Add` (`/Game/FirstPerson/Blueprints/BP_FirstPersonCharacter.Keys` (`self.PlayerRef`)) _keycolorname)
  (`KismetSystemLibrary.PrintString` (`KismetStringLibrary.Concat_StrStr` _keycolorname " key acquired"))
  (`self.K2_DestroyActor`))

(fn `Get_Interact_State`
  (returns (InteractState :type Boolean))
  (return false))

(fn `UserConstructionScript`
  (bind _color (`self.Color`))
  (`PrimitiveComponent.SetMaterial` (`self.key`) 0 (select `/Game/FirstPerson/Blueprints/color` _color :`NewEnumerator0` "/Game/FirstPerson/materials/red.red" :`NewEnumerator1` "/Game/FirstPerson/materials/green.green" :`NewEnumerator2` "/Game/FirstPerson/materials/blue.blue" :!type "MaterialInterface Object Reference"))
  (set `self.KeyColorName` (select `/Game/FirstPerson/Blueprints/color` _color :`NewEnumerator0` "red" :`NewEnumerator1` "green" :`NewEnumerator2` "blue")))