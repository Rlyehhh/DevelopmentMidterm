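; Spike trap actor that applies spike damage to the first-person player character when it begins overlapping the trap.
; On BeginPlay it finds the Spike_Trap_Disabler actor and binds to its traps-disabled event, destroying itself when that fires.
; The construction script sizes the box and cube from the parent BP_Platfrom_Cell's grid size, keeping them flat and slightly inset, when placed as a child actor.
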(event `self.ReceiveBeginPlay`
  (bind _returnvalue (`GameplayStatics.GetActorOfClass` "/Game/Blueprintler/Spike_Trap_Disabler.Spike_Trap_Disabler_C"))
  (add `/Game/Blueprintler/Spike_Trap_Disabler.Traps_Disabled` _returnvalue (delegate `disabled`)))

(event `disabled`
  (`self.K2_DestroyActor`))

(event `self.ReceiveActorBeginOverlap`
  (params (OtherActor :type "Actor Object Reference"))
  (bind _asbp_first_person_character (cast `/Game/FirstPerson/Blueprints/BP_FirstPersonCharacter` OtherActor))
  (bind _output_get (set `self.As BP First Person Character` _asbp_first_person_character))
  (`/Game/FirstPerson/Blueprints/BP_FirstPersonCharacter.Damage_Function` _output_get (`self.Spike_Damage`)))

(fn `UserConstructionScript`
  (bind _asbp_platfrom_cell (cast `/Game/Blueprintler/BP_Platfrom_Cell` (`self.GetParentActor`)))
  (bind _returnvalue (* (`/Game/Blueprintler/BP_Platfrom_Cell.GridSize` _asbp_platfrom_cell) 0.7))
  (`SceneComponent.SetRelativeScale3D` (`self.Box`) (`KismetMathLibrary.MakeVector` _returnvalue _returnvalue 0.1))
  (`SceneComponent.SetRelativeScale3D` (`self.Cube`) (`KismetMathLibrary.MakeVector` _returnvalue _returnvalue 0.1)))